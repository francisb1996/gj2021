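; Staff is an interactable melee weapon that the player picks up and swings.
; On a successful pickup it increments the player's item count, disables its outline, stops its rotating display movement and turns off collision.
; Firing plays a timeline that rotates the hinge for the swing, with an event track running a short camera-forward line trace that damages whatever it hits.
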(event `/Game/Interact.Interact`
  (params (Player :type "/Game/PlayerCharacter Object Reference"))
  (bind _cylinder (`self.Cylinder`))
  (bind _did_pick_up (`/Game/PlayerCharacter.PickUp` Player self))
  (if _did_pick_up
    (`/Game/PlayerCharacter.IncrementItemCount` Player)
    (`self.DisableOutline` self)
    (`SceneComponent.K2_SetRelativeRotation` :`self` _cylinder)
    (`ActorComponent.Deactivate` (`self.RotatingMovement`))
    (`PrimitiveComponent.SetCollisionEnabled` _cylinder "NoCollision")))

(event `/Game/Fire.Fire`
  (params (Player :type "/Game/PlayerCharacter Object Reference"))
  (bind _firstpersoncamera (`/Game/PlayerCharacter.FirstPersonCamera` Player))
  (bind _returnvalue (`SceneComponent.K2_GetComponentLocation` _firstpersoncamera))
  (bind (_direction _newtrack_0) (`Timeline|Timeline_0` :!via `PlayFromStart`)
    (:`Update`
      (`SceneComponent.K2_SetRelativeRotation` (`self.Hinge`) (`KismetMathLibrary.RLerp` (struct) (struct :`Pitch` -90.0 :`Roll` -20.0) _newtrack_0) false false))
    (:`NewTrack_5`
      (bind _outhit (`KismetSystemLibrary.LineTraceSingle` _returnvalue (+ _returnvalue (* (`KismetMathLibrary.GetForwardVector` (`SceneComponent.K2_GetComponentRotation` _firstpersoncamera)) 50.0)) "TraceTypeQuery1" false (`|MakeArray` (`GameplayStatics.GetPlayerCharacter` 0) :!type "Actor Object Reference")))
      (`GameplayStatics.ApplyDamage` (`.HitActor` (`GameplayStatics.BreakHitResult` _outhit)) 10.0))))

(fn `UserConstructionScript`
  (`parent.UserConstructionScript`))