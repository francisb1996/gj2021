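; Bone is an interactable item that the player can pick up and throw as a weapon.
; On pickup it turns off its outline, physics, collision and bending strength.
; Firing plays a short pull-back timeline, then detaches it from the player's weapons and launches it spinning along the camera's forward vector.
; The throw restores collision, physics and bending, and re-enables the outline only if the player has a hat.
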(event `/Game/Interact.Interact`
  (params (Player :type "/Game/PlayerCharacter Object Reference"))
  (bind _staticmesh (`self.StaticMesh`))
  (bind _did_pick_up (`/Game/PlayerCharacter.PickUp` Player self))
  (if _did_pick_up
    (`self.DisableOutline` self)
    (`PrimitiveComponent.SetSimulatePhysics` _staticmesh false)
    (`PrimitiveComponent.SetCollisionEnabled` _staticmesh "NoCollision")
    (set `/Game/PN_LowpolyGras/Blueprints/PN_Bending_Component.Bending Strength Scale` 0.0 (`self.PN_Bending_Component`))))

(event `/Game/Fire.Fire`
  (params (Player :type "/Game/PlayerCharacter Object Reference"))
  (bind _staticmesh (`self.StaticMesh`))
  (bind (_direction _newtrack_0) (`Timeline|Throw` :!via `PlayFromStart`)
    (:`Update`
      (`SceneComponent.K2_SetRelativeLocation` (`self.StaticMesh`) (`KismetMathLibrary.VLerp` (0.0 0.0 0.0) (-20.0 0.0 0.0) _newtrack_0) false false))
    (:`Finished`
      (`self.K2_DetachFromActor` "KeepWorld" "KeepWorld" "KeepWorld")
      (`/Game/PlayerCharacter.RemoveWeapon` Player (`/Game/PlayerCharacter.WeaponIndex` Player))
      (`PrimitiveComponent.SetCollisionEnabled` _staticmesh "QueryAndPhysics")
      (`PrimitiveComponent.SetSimulatePhysics` _staticmesh true)
      (`PrimitiveComponent.AddImpulse` _staticmesh (* (`SceneComponent.GetForwardVector` (`/Game/PlayerCharacter.FirstPersonCamera` Player)) 1000.0) "None" true)
      (`PrimitiveComponent.AddTorqueInDegrees` (`self.StaticMesh`) (50000.0 0.0 0.0) "None" true)
      (`PrimitiveComponent.AddTorqueInDegrees` _staticmesh (50000.0 0.0 0.0) "None" true)
      (set `/Game/PN_LowpolyGras/Blueprints/PN_Bending_Component.Bending Strength Scale` 1.5 (`self.PN_Bending_Component`))
      (if (`/Game/PlayerCharacter.HasHat` Player)
        (`self.EnableOutline` self)))))

(fn `UserConstructionScript`)